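; BP_PorteUn is a door Blueprint that slides its static mesh between a closed and an open position.
; On BeginPlay it binds its Activation event to the EventLauncher's controlables dispatcher.
; Activation, Activate and Desactivate all call OpenClose, so each acts as a toggle.
; OpenClose checks the mesh's relative X, snaps it to the opposite position without interpolation, and prints a debug string.
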(event `self.ReceiveBeginPlay`
  (add `/Game/ElementsDevoir/BP_InterrupteurUn.Activate Controlables` (`self.Event Launcher`) (delegate `Activation`)))

(event `Activation`
  (`self.Open Close`))

(event `/Game/ElementsDevoir/BPI_Interrupeurs.Activate`
  (`self.Open Close`))

(event `/Game/ElementsDevoir/BPI_Interrupeurs.Desactivate`
  (`self.Open Close`))

(fn `Open Close`
  (bind _relativelocation_x (`KismetMathLibrary.BreakVector` (`SceneComponent.RelativeLocation` (`self.StaticMesh`))))
  (if (>= _relativelocation_x 10.0)
    (`KismetSystemLibrary.PrintString` "Bruh")
    (`SceneComponent.K2_SetRelativeLocation` (`self.StaticMesh`) (0.0 0.0 0.0) false false)
    (else
      (`KismetSystemLibrary.PrintString` "AAA")
      (`SceneComponent.K2_SetRelativeLocation` (`self.StaticMesh`) (100.0 0.0 0.0) false false))))

(fn `UserConstructionScript`)