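; BP_Lampe is a lamp actor whose light component can be switched on and off.
; On BeginPlay it binds its Activation event to the ActivateControlables event of an EventLauncher.
; Activation, Activate and Desactivate all call ToggleLight, which inverts the visibility of the Lumiere component, so Activate and Desactivate flip the current state rather than setting it explicitly.
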(event `self.ReceiveBeginPlay`
  (add `/Game/ElementsDevoir/BP_InterrupteurUn.Activate Controlables` (`self.Event Launcher`) (delegate `Activation`)))

(event `Activation`
  (`self.ToggleLight`))

(event `/Game/ElementsDevoir/BPI_Interrupeurs.Activate`
  (`self.ToggleLight`))

(event `/Game/ElementsDevoir/BPI_Interrupeurs.Desactivate`
  (`self.ToggleLight`))

(fn `ToggleLight`
  (bind _lumiere (`self.Lumiere`))
  (`SceneComponent.SetVisibility` _lumiere (not (`SceneComponent.bVisible` _lumiere)) false))

(fn `UserConstructionScript`)